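; World manager Blueprint that signals when world generation is complete and populates chunks with enemies.
; Tick calls the world-generated event once, after IsGenerated becomes true.
; SpawnEnemiesfromChunk has a 50% chance to roll among Smile, Zombunny, Hellephant or no spawn, placing the enemy at a random inset point in the chunk.
; It then moves the enemy to a surface floor position found from a separately randomized point.
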(event `self.ReceiveTick`
  (params (DeltaSeconds :type "Float (single-precision)"))
  (if (`self.IsGenerated`)
    (`/Engine/EditorBlueprintResources/StandardMacros.DoOnce` false
      (:`Completed`
        (`self.WorldGeneratedEvent`)))))

(event `self.SpawnEnemiesFromChunk`
  (params (ChunkPos :type "Vector Structure"))
  (bind _blocksize (`self.BlockSize`))
  (bind _chunkwidth (`self.ChunkWidth`))
  (bind _returnvalue (* _blocksize (* _chunkwidth 0.1)))
  (bind _returnvalue_2 (`KismetMathLibrary.RandomFloatInRange` _returnvalue (- (* _chunkwidth _blocksize) _returnvalue)))
  (bind _returnvalue_3 (+ ChunkPos (`KismetMathLibrary.MakeVector` _returnvalue_2 _returnvalue_2)))
  (bind _returnvalue_4 (`KismetMathLibrary.Conv_VectorToVector2D` _returnvalue_3))
  (if (< (`KismetMathLibrary.RandomFloat`) 0.5)
    (switch `int` (`KismetMathLibrary.RandomInteger` 4)
      (:`0`
        (bind _returnvalue_5 (`|SpawnActorFromClass` "/Game/Blueprints/Character/Enemy/BP_Smile.BP_Smile_C" (`KismetMathLibrary.MakeTransform` _returnvalue_3) "DontSpawnIfColliding" "OverrideRootScale" null null))
        (bind (_radius_size_x _radius_size_y _radius_size_z) (`KismetMathLibrary.BreakVector` (`/Game/Blueprints/Character/Enemy/Base/BP_Enemy_Simple.Radius Size` _returnvalue_5)))
        (`self.K2_SetActorLocation` _returnvalue_5 (`self.GetSurfaceFloorPos` _returnvalue_4 _radius_size_x _radius_size_y _radius_size_z) false false))
      (:`1`
        (bind _returnvalue_6 (`|SpawnActorFromClass` "/Game/Blueprints/Character/Enemy/BP_Zombunny.BP_Zombunny_C" (`KismetMathLibrary.MakeTransform` _returnvalue_3) "DontSpawnIfColliding" "OverrideRootScale" null null))
        (`self.K2_SetActorLocation` _returnvalue_6 (`self.GetSurfaceFloorPos` _returnvalue_4 1.0 1.0 1.0) false false))
      (:`2`
        (bind _returnvalue_7 (`|SpawnActorFromClass` "/Game/Blueprints/Character/Enemy/BP_Hellephant.BP_Hellephant_C" (`KismetMathLibrary.MakeTransform` _returnvalue_3) "DontSpawnIfColliding" "OverrideRootScale" null null))
        (`self.K2_SetActorLocation` _returnvalue_7 (`self.GetSurfaceFloorPos` _returnvalue_4 1.0 1.0 1.0) false false)))))

(fn `UserConstructionScript`)