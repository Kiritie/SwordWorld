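; BP_Enemy_Simple is a simple base enemy Blueprint with health, patrol targeting and a hit response hook.
; It caches the player character on BeginPlay and creates a dynamic material for its body in construction.
; Helpers clamp health and update the death flag, pick random patrol points around the current location, and measure horizontal distance to that target.
; HitWithAttack is a stub that returns true without applying damage.
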(event `self.ReceiveBeginPlay`
  (bind _asbp_player_character (cast `/Game/Blueprints/Character/Player/BP_PlayerCharacter` (`GameplayStatics.GetPlayerCharacter` 0)))
  (set `self.Player Character` _asbp_player_character))

(fn `Get Distance To Target Pos`
  (returns (Distance :type "Float (double-precision)"))
  (bind (_returnvalue_x _returnvalue_y) (`KismetMathLibrary.BreakVector` (- (`self.K2_GetActorLocation`) (`self.Move Target Pos`))))
  (return (`KismetMathLibrary.VSize` (`KismetMathLibrary.MakeVector` _returnvalue_x _returnvalue_y))))

(fn `Hit with attack`
  (params (`Repelled vector` :type "Vector Structure") (`Damage value` :type "Float (double-precision)") (Attacker :type "Actor Object Reference"))
  (returns (bWasDamaged :type Boolean))
  (return true))

(fn `Modify Health`
  (params (Value :type "Float (double-precision)") (Addition :type Boolean :default true))
  (bind _current_health (`self.Current Health`))
  (bind _maximum_health (`self.Maximum Health`))
  (if Addition
    (set `self.Current Health` (`KismetMathLibrary.FClamp` (+ _current_health Value) 0.0 _maximum_health))
    (else
      (set `self.Current Health` (`KismetMathLibrary.FClamp` (- _current_health Value) 0.0 _maximum_health))))
  (set `self.Is Dead` (<= (`self.Current Health`) 0.0)))

(fn `Random Target Pos`
  (set `self.Move Target Pos` (+ (`self.K2_GetActorLocation`) (`KismetMathLibrary.GreaterGreater_VectorRotator` (`KismetMathLibrary.MakeVector` (* (`KismetMathLibrary.RandomFloatInRange` 0.7 1.0) (`self.Patrolling Range`))) (`KismetMathLibrary.MakeRotator` 0.0 0.0 (`KismetMathLibrary.RandomFloatInRange` 0.0 360.0))))))

(fn `UserConstructionScript`
  (bind _returnvalue (`PrimitiveComponent.CreateDynamicMaterialInstance` (`self.Body`) 0 null "None"))
  (set `self.Body MID` _returnvalue))