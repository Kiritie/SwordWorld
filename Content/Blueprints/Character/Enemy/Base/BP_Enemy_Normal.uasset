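; Base melee enemy character that patrols random points, chases the player within sight range and attacks on a timed cooldown.
; Tick steers with direct movement input rather than navigation, and when AutoJump is off, a low forward trace jumps it over Chunk obstacles.
; Attacks go through a hit message whose return selects a stab or blocked sound.
; Incoming hits apply damage, notify the attacker, and on death award experience before delayed destruction.
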(event `self.ReceiveBeginPlay`
  (bind _asbp_player_character (cast `/Game/Blueprints/Character/Player/BP_PlayerCharacter` (`GameplayStatics.GetPlayerCharacter` 0)))
  (set `self.Player Character` _asbp_player_character))

(event `self.ReceiveTick`
  (params (DeltaSeconds :type "Float (single-precision)"))
  (bind (_returnvalue_x _returnvalue_y _returnvalue_z) (`KismetMathLibrary.BreakVector` (`self.K2_GetActorLocation`)))
  (bind _sight_distance (`self.Sight Distance`))
  (bind _attack_target (`self.Attack Target`))
  (bind _player_character (`self.Player Character`))
  (bind _attack_target_2 (`self.Attack Target`))
  (bind _capsulecomponent (`self.CapsuleComponent`))
  (bind (_returnvalue_roll _returnvalue_pitch _returnvalue_yaw) (`KismetMathLibrary.BreakRotator` (`KismetMathLibrary.FindLookAtRotation` (`self.K2_GetActorLocation`) (`self.Move Target Pos`))))
  (bind _returnvalue (`self.K2_GetActorLocation` _attack_target))
  (bind _dead (`/Game/Blueprints/Character/Player/BP_PlayerCharacter.Dead` (`self.Player Character`)))
  (bind _returnvalue_2 (and (`KismetSystemLibrary.IsValid` (`self.Attack Target`)) (<= (`self.Get Distance To Target Pos`) (`self.Attack Distance`))))
  (bind _returnvalue_3 (`KismetMathLibrary.MakeVector` _returnvalue_x _returnvalue_y (- _returnvalue_z (- (`CapsuleComponent.GetScaledCapsuleHalfHeight` _capsulecomponent) (`CharacterMovementComponent.MaxStepHeight` (`self.CharacterMovement`))))))
  (if (`self.Is Dead`)
    _
    (elif (`self.Is Patrolling`)
      (`|ExecutionSequence`
        (:`then_0`
          (`/Engine/EditorBlueprintResources/StandardMacros.IsValid` (`self.Attack Target`)
            (:`Is Valid`
              (if (or (> (`self.GetDistanceTo` _attack_target_2) _sight_distance) (and (== _attack_target_2 _player_character) _dead))
                (set `self.Attack Target` (`self.NewVar_0`))
                (`self.Random Target Pos`)
                (else
                  (set `self.Move Target Pos` (`self.K2_GetActorLocation` (`self.Attack Target`))))))
            (:`Is Not Valid`
              (if (and (<= (`self.GetDistanceTo` _player_character) _sight_distance) (not _dead))
                (set `self.Attack Target` (`self.Player Character`))
                (elif (<= (`self.Get Distance To Target Pos`) 50.0)
                  (`self.Random Target Pos`))))))
        (:`then_1`
          (if (not _returnvalue_2)
            (set `CharacterMovementComponent.MaxWalkSpeed` (`self.Movement Speed`) (`self.CharacterMovement`))
            (`self.AddMovementInput` (`self.Get Direction To Target Pos`))
            (`|ExecutionSequence`
              (:`then_0`
                (if (not (`self.Auto Jump`))
                  (bind _outhit (`KismetSystemLibrary.LineTraceSingle` _returnvalue_3 (+ _returnvalue_3 (* (`self.GetActorForwardVector`) (+ (`CapsuleComponent.GetScaledCapsuleRadius` _capsulecomponent) 30.0))) "TraceTypeQuery1"))
                  (cast `Chunk` (`.HitActor` (`GameplayStatics.BreakHitResult` _outhit)))
                  (`self.Jump`)))
              (:`then_1`
                (`/Engine/EditorBlueprintResources/StandardMacros.DoOnce` false
                  (:`Completed`
                    (set `self.Attack Countdown` (/ 0.5 (`self.Attack Speed`)))))))))
        (:`then_2`
          (if _returnvalue_2
            (`self.K2_SetActorRotation` (`KismetMathLibrary.MakeRotator` 0.0 0.0 _returnvalue_yaw))
            (bind _output_get (set `self.Attack Countdown` (- (`self.Attack Countdown`) (`GameplayStatics.GetWorldDeltaSeconds`))))
            (if (<= _output_get 0.0)
              (bind _bwasdamaged (message `/Game/Blueprints/Character/Player/Base/BPI_Weapon_Interactions.Hit with attack` _attack_target (0.0 0.0 0.0) (`self.Attack Damage`) self))
              (set `self.Attack Countdown` (/ 1.0 (`self.Attack Speed`)))
              (if _bwasdamaged
                (`GameplayStatics.PlaySoundAtLocation` "/Game/Sounds/Sword_Stab06.Sword_Stab06" _returnvalue (struct) 1.0 1.0 0.0 null null null)
                (else
                  (`GameplayStatics.PlaySoundAtLocation` "/Game/Sounds/Attack_Blocked.Attack_Blocked" _returnvalue (struct) 1.0 1.0 0.0 null null null))))))))))

(event `self.ReceiveAnyDamage`
  (params (Damage :type "Float (single-precision)") (DamageType :type "DamageType Object Reference") (InstigatedBy :type "Controller Object Reference") (DamageCauser :type "Actor Object Reference"))
  (`self.Modify Health` Damage false)
  (message `/Game/Blueprints/Character/Player/Base/BPI_Weapon_Interactions.Enemy attacked` DamageCauser Damage)
  (if (`self.Is Dead`)
    (message `/Game/Blueprints/Character/Player/Base/BPI_Weapon_Interactions.Enemy killed` DamageCauser (`self.K2_GetActorLocation`) 50.0)
    (`PrimitiveComponent.SetCollisionEnabled` (`self.CapsuleComponent`) "NoCollision")
    (`KismetSystemLibrary.Delay` 1.5)
    (`self.K2_DestroyActor`)))

(fn `Get Direction To Target Pos`
  (returns (Direction :type "Vector Structure"))
  (bind (_returnvalue_x _returnvalue_y) (`KismetMathLibrary.BreakVector` (`KismetMathLibrary.GetDirectionUnitVector` (`self.K2_GetActorLocation`) (`self.Move Target Pos`))))
  (return (`KismetMathLibrary.Normal` (`KismetMathLibrary.MakeVector` _returnvalue_x _returnvalue_y))))

(fn `Get Distance To Target Pos`
  (returns (Distance :type "Float (double-precision)"))
  (return (`KismetMathLibrary.VSize` (- (`self.K2_GetActorLocation`) (`self.Move Target Pos`)))))

(fn `Hit with attack`
  (params (`Repelled vector` :type "Vector Structure") (`Damage value` :type "Float (double-precision)") (Attacker :type "Actor Object Reference"))
  (returns (bWasDamaged :type Boolean))
  (`GameplayStatics.ApplyDamage` self `Damage value` null Attacker)
  (return true))

(fn `Modify Health`
  (params (Value :type "Float (double-precision)") (Addition :type Boolean :default true))
  (bind _current_health (`self.Current Health`))
  (bind _maximum_health (`self.Maximum Health`))
  (if Addition
    (set `self.Current Health` (`KismetMathLibrary.FClamp` (+ _current_health Value) 0.0 _maximum_health))
    (else
      (set `self.Current Health` (`KismetMathLibrary.FClamp` (- _current_health Value) 0.0 _maximum_health))))
  (set `self.Is Dead` (<= (`self.Current Health`) 0.0)))

(fn `Random Target Pos`
  (set `self.Move Target Pos` (+ (`self.K2_GetActorLocation`) (`KismetMathLibrary.GreaterGreater_VectorRotator` (`KismetMathLibrary.MakeVector` (* (`KismetMathLibrary.RandomFloatInRange` 0.7 1.0) (`self.Patrolling Range`))) (`KismetMathLibrary.MakeRotator` 0.0 0.0 (`KismetMathLibrary.RandomFloatInRange` 0.0 360.0))))))

(fn `UserConstructionScript`
  (bind _returnvalue (`PrimitiveComponent.CreateDynamicMaterialInstance` (`self.Mesh`) 0 null "None"))
  (set `self.Body MID` _returnvalue))