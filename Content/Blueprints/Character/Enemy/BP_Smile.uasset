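; Bouncing enemy that hops between random patrol points and chases the living player while within sight range.
; Tick simulates gravity with swept offsets, relaunching on each upward-facing impact and sending an attack to whatever it lands on.
; It turns toward its target and moves forward only while jumping.
; Damage lowers health and notifies the attacker; death fades the body material, destroys the actor and reports experience to the killer.
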(event `self.ReceiveBeginPlay`
  (`parent.ReceiveBeginPlay`))

(event `self.ReceiveTick`
  (params (DeltaSeconds :type "Float (single-precision)"))
  (bind _player_character (`self.Player Character`))
  (bind _sight_distance (`self.Sight Distance`))
  (bind _attack_target (`self.Attack Target`))
  (bind (_returnvalue_roll _returnvalue_pitch _returnvalue_yaw) (`KismetMathLibrary.BreakRotator` (`KismetMathLibrary.FindLookAtRotation` (`self.K2_GetActorLocation`) (`self.Move Target Pos`))))
  (bind _dead (`/Game/Blueprints/Character/Player/BP_PlayerCharacter.Dead` (`self.Player Character`)))
  (if (not (`self.Is Dead`))
    (`|ExecutionSequence`
      (:`then_0`
        (bind _sweephitresult (`self.K2_AddActorWorldOffset` (`KismetMathLibrary.MakeVector` 0.0 0.0 (* (`self.Movement Speed Z Axis`) (`GameplayStatics.GetWorldDeltaSeconds`))) true))
        (`|ExecutionSequence`
          (:`then_0`
            (bind (_bblockinghit _binitialoverlap _time _distance _location _impactpoint _normal _impactnormal _physmat _hitactor) (`GameplayStatics.BreakHitResult` _sweephitresult))
            (bind _z (.z _impactnormal))
            (if (> _z 0.0)
              (set `self.Movement Speed Z Axis` (`self.Jump Speed`))
              (set `self.Is Jumping` true)
              (`/Engine/EditorBlueprintResources/StandardMacros.IsValid` _hitactor
                (:`Is Valid`
                  (bind _bwasdamaged (message `/Game/Blueprints/Character/Player/Base/BPI_Weapon_Interactions.Hit with attack` _hitactor (0.0 0.0 0.0) 100.0 self))
                  (if _bwasdamaged
                    (`GameplayStatics.PlaySoundAtLocation` "/Game/Sounds/Sword_Stab06.Sword_Stab06" _impactpoint (struct) 1.0 1.0 0.0 null null null))))))
          (:`then_1`
            (if (< _z 0.0)
              (set `self.Movement Speed Z Axis` 0.0)
              (set `self.Is Jumping` false)))
          (:`then_2`
            (set `self.Movement Speed Z Axis` (- (`self.Movement Speed Z Axis`) (* (`self.Gravity Value`) (`GameplayStatics.GetWorldDeltaSeconds`)))))))
      (:`then_1`
        (if (`self.Is Patrolling`)
          (if (> (`self.Get Distance To Target Pos`) 20.0)
            (`self.K2_SetActorRotation` (`KismetMathLibrary.RLerp` (`self.K2_GetActorRotation`) (`KismetMathLibrary.MakeRotator` 0.0 0.0 _returnvalue_yaw) (* (`GameplayStatics.GetWorldDeltaSeconds`) 10.0) true))
            (if (`self.Is Jumping`)
              (`self.K2_AddActorWorldOffset` (* (`self.GetActorForwardVector`) (* (`self.Movement Speed X Axis`) (`GameplayStatics.GetWorldDeltaSeconds`))) true)))))
      (:`then_2`
        (`/Engine/EditorBlueprintResources/StandardMacros.IsValid` (`self.Attack Target`)
          (:`Is Valid`
            (if (or (> (`self.GetDistanceTo` _attack_target) _sight_distance) (and (== _attack_target _player_character) _dead))
              (set `self.Attack Target` (`self.NewVar_0_0`))
              (`self.Random Target Pos`)
              (else
                (set `self.Move Target Pos` (`self.K2_GetActorLocation` (`self.Attack Target`))))))
          (:`Is Not Valid`
            (if (and (<= (`self.GetDistanceTo` _player_character) _sight_distance) (not _dead))
              (set `self.Attack Target` (`self.Player Character`))
              (elif (<= (`self.Get Distance To Target Pos`) 50.0)
                (`self.Random Target Pos`)))))))))

(event `self.ReceiveAnyDamage`
  (params (Damage :type "Float (single-precision)") (DamageType :type "DamageType Object Reference") (InstigatedBy :type "Controller Object Reference") (DamageCauser :type "Actor Object Reference"))
  (`self.Modify Health` Damage false)
  (message `/Game/Blueprints/Character/Player/Base/BPI_Weapon_Interactions.Enemy attacked` DamageCauser Damage)
  (if (`self.Is Dead`)
    (`KismetSystemLibrary.Delay` 0.1)
    (bind (_direction _opacity) (`Timeline|OpacityChange_TimeLine`)
      (:`Update`
        (`MaterialInstanceDynamic.SetScalarParameterValue` (`self.Body MID`) "Opacity" _opacity))
      (:`Finished`
        (`self.K2_DestroyActor`)
        (message `/Game/Blueprints/Character/Player/Base/BPI_Weapon_Interactions.Enemy killed` DamageCauser (`self.K2_GetActorLocation`) 50.0)))))

(fn `Hit with attack`
  (params (`Repelled vector` :type "Vector Structure") (`Damage value` :type "Float (double-precision)") (Attacker :type "Actor Object Reference"))
  (returns (bWasDamaged :type Boolean))
  (`GameplayStatics.ApplyDamage` self `Damage value`)
  (return true))

(fn `UserConstructionScript`
  (`parent.UserConstructionScript`))