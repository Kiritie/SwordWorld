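; Player fireball projectile that launches along its facing direction with an attached sound and destroys itself after a fixed lifetime.
; WeaponCollision overlaps that pass a Chunk cast destroy it early, then apply heavy damage credited to its owner if that actor also casts to BP_Enemy_Simple.
; The enemy check is nested inside the Chunk check, and HitWithAttack is a stub returning false.
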(event `self.ReceiveBeginPlay`
  (set `MovementComponent.Velocity` (`KismetMathLibrary.GreaterGreater_VectorRotator` (`self.Initial Velocity`) (`self.K2_GetActorRotation`)) (`self.Projectile component`))
  (`GameplayStatics.SpawnSoundAttached` "/Game/Audio/Room_03/Arcade_Enemy_Destroyed_Cue.Arcade_Enemy_Destroyed_Cue" (`self.Fireball`) "None" (0.0 0.0 0.0) (struct) "KeepRelativeOffset" false 1.0 1.0 0.0 null null)
  (`KismetSystemLibrary.Delay` 10.0)
  (`self.K2_DestroyActor`))

(event `self.Weapon collision.OnComponentBeginOverlap`
  (params (OverlappedComponent :type "PrimitiveComponent Object Reference") (OtherActor :type "Actor Object Reference") (OtherComp :type "PrimitiveComponent Object Reference") (OtherBodyIndex :type Integer) (bFromSweep :type Boolean) (SweepResult :type "HitResult Structure (by ref)"))
  (bind (_asbp_enemy_simple _bsuccess) (cast `/Game/Blueprints/Character/Enemy/Base/BP_Enemy_Simple` OtherActor :!pure true))
  (if (or (`.bSuccess` (cast `Chunk` OtherActor :!pure true)) false)
    (`self.K2_DestroyActor`)
    (if _bsuccess
      (`GameplayStatics.ApplyDamage` _asbp_enemy_simple 200.0 null (`self.Owner_0`)))))

(fn `Hit with attack`
  (params (`Impact vector` :type "Vector Structure") (`Weapon damage` :type "Float (double-precision)") (`Weapon weight` :type "Float (double-precision)") (Attacker :type "Actor Object Reference"))
  (returns (bWasDamaged :type Boolean))
  (return false))

(fn `UserConstructionScript`)